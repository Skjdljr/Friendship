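; BPA_Bullet is a projectile actor that flies toward the Crosshair component of a Ship reference.
; On BeginPlay it sets the crosshair as the ProjectileMovement homing target.
; Each Tick it also turns to face the crosshair and rebuilds velocity along that heading at the current speed, tracking the crosshair as it moves.
; It destroys itself when its Plane component nearly reaches the crosshair or when projectile movement stops.
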(event `self.ReceiveBeginPlay`
  (set `ProjectileMovementComponent.HomingTargetComponent` (`/Game/Blueprints/BPA_TheFriendship.Crosshair` (`self.ship`)) (`self.ProjectileMovement`)))

(event `self.ReceiveTick`
  (params (DeltaSeconds :type "Float (single-precision)"))
  (bind (_returnvalue_roll _returnvalue_pitch _returnvalue_yaw) (`KismetMathLibrary.BreakRotator` (`self.K2_GetActorRotation`)))
  (`self.K2_SetActorRotation` (`KismetMathLibrary.FindLookAtRotation` (`self.K2_GetActorLocation`) (`SceneComponent.K2_GetComponentLocation` (`/Game/Blueprints/BPA_TheFriendship.Crosshair` (`self.ship`)))))
  (set `MovementComponent.Velocity` (`KismetMathLibrary.CreateVectorFromYawPitch` _returnvalue_yaw _returnvalue_pitch (`KismetMathLibrary.VSize` (`self.GetVelocity`))) (`self.ProjectileMovement`))
  (if (== (`SceneComponent.K2_GetComponentLocation` (`self.Plane`)) (`SceneComponent.K2_GetComponentLocation` (`/Game/Blueprints/BPA_TheFriendship.Crosshair` (`self.ship`))) :`ErrorTolerance` 16.0)
    (`self.K2_DestroyActor`)))

(event `self.ProjectileMovement.OnProjectileStop`
  (params (ImpactResult :type "HitResult Structure (by ref)"))
  (`self.K2_DestroyActor`))

(fn `UserConstructionScript`)