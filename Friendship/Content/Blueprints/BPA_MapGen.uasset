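; BPA_MapGen procedurally builds a map at BeginPlay by chaining piece actors from a start piece to an end piece.
; Random left, right or straight pieces spawn at a previous piece's connection point until MapLength, with an optional delay to watch progress.
; Pieces flagging NeedRespawn are destroyed and their class excluded; dead ends trigger backtracking, deeper after repeated failures.
; Completion calls CallGenFinished and prints the load time accumulated on Tick.
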(event `self.ReceiveBeginPlay`
  (bind _pieces (`self.Pieces`))
  (bind _tempclasses (`self.TempClasses`))
  (bind _returnvalue (`KismetArrayLibrary.Array_Length` (`self.Pieces`)))
  (bind _returnvalue_2 (- (`KismetArrayLibrary.Array_Length` (`self.Pieces`)) 1))
  (bind _returnvalue_3 (- (`KismetArrayLibrary.Array_Length` (`self.Pieces`)) 1))
  (bind _returnvalue_4 (`|SpawnActorFromClass` "/Game/Blueprints/BPA_Start.BPA_Start_C" (`KismetMathLibrary.MakeTransform` (0.0 0.0 0.0)) "Undefined" "OverrideRootScale" null 0 null)) ; Spawn the Start
  (`KismetArrayLibrary.Array_Add` (`self.Pieces`) _returnvalue_4)
  (set `self.TempClasses` (`self.MapClasses`) :!label _label) ; All the Possible Choices
  ;[0 1 0.03028] Spawn Pieces
  (if (> (`KismetArrayLibrary.Array_Length` (`self.TempClasses`)) 0) :!label _label_2
    (if (== _returnvalue (- (`self.MapLength`) 1))
      (bind _output_get (set `self.RandoClass` "/Game/Blueprints/BPA_End.BPA_End_C"))
      (set `self.TempClasses` (`|MakeArray` _output_get)) ; Only want the end, still want to test if its valid
      (else
        (set `self.RandoClass` (`|GetArrayItem` _tempclasses (`KismetMathLibrary.RandomInteger` (`KismetArrayLibrary.Array_Length` _tempclasses))))))
    (bind _returnvalue_5 (`|SpawnActorFromClass` (`self.RandoClass`) (`SceneComponent.K2_GetComponentToWorld` (`/Game/Blueprints/BPA_Map_Base.ConnectionPoint` (`|GetArrayItem` (`self.Pieces`) (- (`self.Current`) (select `bool` (> (`self.fails`) 0) :`false` 1))))) "Undefined" "OverrideRootScale" null _returnvalue null)) ; Spawn it and hope for the best
    (if (`/Game/Blueprints/BPA_Map_Base.needRespawn` _returnvalue_5)
      (`self.K2_DestroyActor` _returnvalue_5) ; It did, kill it
      (`KismetArrayLibrary.Array_RemoveItem` (`self.TempClasses`) (`self.RandoClass`)) ; This type won't work, don't try again
      (goto _label_2)
      (else
        (`KismetArrayLibrary.Array_Add` (`self.Pieces`) _returnvalue_5)
        (set `self.MapClasses` (`|MakeArray` "/Game/Blueprints/BPA_Left.BPA_Left_C" "/Game/Blueprints/BPA_Right.BPA_Right_C" "/Game/Blueprints/BPA_Straight.BPA_Straight_C" :!type "/Game/Blueprints/BPA_Map_Base Class Reference")) ; Successfully added a piece, reset mapclases
        (set `self.Current` (+ (`self.Current`) 1))
        ;[1 0.8187 0.07785] Stop if we hit Max Length
        (if (== (`KismetArrayLibrary.Array_Length` (`self.Pieces`)) (`self.MapLength`))
          (`self.GenFinished`)
          (`self.SetActorTickEnabled` false)
          (`KismetSystemLibrary.PrintString` (`KismetStringLibrary.Conv_DoubleToString` (`self.LoadTime`)))
          (else
            (`KismetSystemLibrary.Delay` (`self.SpawnDelay`) :!label _label_3) ; Delay if to add things slowly to watch it working
            (goto _label)))))
    (else
      ;[1 0 0] Dead end
      (if (and (!= (`KismetArrayLibrary.Array_Length` (`self.Pieces`)) (+ (`self.MapLength`) 1)) (< (`self.fails`) 3))
        (`KismetArrayLibrary.Array_RemoveItem` (`self.MapClasses`) (`self.RandoClass`)) ; The random piece will never work, stop trying
        (`/Engine/EditorBlueprintResources/StandardMacros.IncrementInt` (`self.fails`) ; Keep track of how many times a piece couldn't be placed
          (:`  `
            _))
        (else
          (set `self.fails` 0) ; Too deep in the dead end
          (`self.K2_DestroyActor` (`|GetArrayItem` _pieces _returnvalue_3)) ; Delete this peiece, and will later delete the previous piece since nothing can be placed anymore, will start over with hopefully a new random piece
          (`KismetArrayLibrary.Array_Remove` _pieces _returnvalue_3)
          (set `self.MapClasses` (`|MakeArray` "/Game/Blueprints/BPA_Left.BPA_Left_C" "/Game/Blueprints/BPA_Right.BPA_Right_C" "/Game/Blueprints/BPA_Straight.BPA_Straight_C" :!type "/Game/Blueprints/BPA_Map_Base Class Reference")) ; Backing out of this piece, we can try all types again
        ))
      (`self.K2_DestroyActor` (`|GetArrayItem` (`self.Pieces`) _returnvalue_2)) ; The Piece lead to a dead end, remove it
      (`KismetArrayLibrary.Array_Remove` (`self.Pieces`) _returnvalue_2)
      (set `self.Current` _returnvalue_2)
      (goto _label_3))))

(event `self.ReceiveTick`
  (params (DeltaSeconds :type "Float (single-precision)"))
  (set `self.LoadTime` (+ DeltaSeconds (`self.LoadTime`))))

(fn `UserConstructionScript`)