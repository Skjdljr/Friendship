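; BPA_TheFriendship is the player-controlled spaceship, with twin engines, a turret and a Box overlap that returns to MainMenu.
; Adjustable left/right engine power drives radial forces, differential yaw and plume scale, while front thrusters push using timer-replenished energy.
; The turret follows a clamped crosshair and fires BPA_Bullet after a reload on the randomly chosen side.
; A wrong-side or repeated reload jams reloading briefly and rerolls the side.
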(event `self.ReceiveBeginPlay`
  (`self.ChooseBulletSide`)
  (`KismetSystemLibrary.K2_SetTimerDelegate` (delegate `OnTimerComplete`) 3.0 true))

(event `OnTimerComplete`
  (`self.AccumulateThrusterEnergy` 5))

(event `self.ReceiveTick`
  (params (DeltaSeconds :type "Float (single-precision)"))
  (`PrimitiveComponent.AddRadialForce` (`self.Ship`) (`SceneComponent.K2_GetComponentLocation` (`self.RightEngine`)) 50.0 (`self.RightPower`) "RIF_Constant" false)
  (`PrimitiveComponent.AddRadialForce` (`self.Ship`) (`SceneComponent.K2_GetComponentLocation` (`self.LeftEngine`)) 50.0 (`self.LeftPower`) "RIF_Constant" false)
  (`SceneComponent.K2_AddWorldRotation` (`self.Ship`) (`KismetMathLibrary.MakeRotator` 0.0 0.0 (/ (- (`self.LeftPower`) (`self.RightPower`)) 20.0)) false false)
  (`SceneComponent.SetRelativeScale3D` (`self.LeftThrustRoot`) (`KismetMathLibrary.MakeVector` 0.2 (`KismetMathLibrary.MapRangeClamped` (`self.LeftPower`) 1.0 10.0 0.1 0.5) 0.8))
  (`SceneComponent.SetRelativeScale3D` (`self.RightThrustRoot`) (`KismetMathLibrary.MakeVector` 0.2 (`KismetMathLibrary.MapRangeClamped` (`self.RightPower`) 1.0 10.0 0.1 0.5) 0.8)))

(event `InputAxis|PowerUpRight`
  (params (AxisValue :type "Float (single-precision)"))
  (set `self.RightPower` (`KismetMathLibrary.FClamp` (+ AxisValue (`self.RightPower`)) 1.0 10.0)))

(event `InputAxis|PowerDownRight`
  (params (AxisValue :type "Float (single-precision)"))
  (set `self.RightPower` (`KismetMathLibrary.FClamp` (- (`self.RightPower`) AxisValue) 1.0 10.0)))

(event `InputAxis|CrosshairX`
  (params (AxisValue :type "Float (single-precision)"))
  (bind _turret (`self.Turret`))
  (bind (_relativelocation_x _relativelocation_y) (`KismetMathLibrary.BreakVector` (`SceneComponent.RelativeLocation` (`self.Crosshair`))))
  (if (and (< _relativelocation_x 300.0) (> _relativelocation_x -300.0) (not (`self.Fired`)))
    (`SceneComponent.K2_SetRelativeLocation` (`self.Crosshair`) (`KismetMathLibrary.MakeVector` (`KismetMathLibrary.FClamp` (+ _relativelocation_x AxisValue) -300.0 300.0) _relativelocation_y) false false)
    (`SceneComponent.K2_SetRelativeRotation` _turret (`KismetMathLibrary.FindLookAtRotation` (`SceneComponent.RelativeLocation` _turret) (`SceneComponent.RelativeLocation` (`self.Crosshair`))) false false :!label _label)))

(event `InputAxis|PowerUpLeft`
  (params (AxisValue :type "Float (single-precision)"))
  (set `self.LeftPower` (`KismetMathLibrary.FClamp` (+ AxisValue (`self.LeftPower`)) 1.0 10.0)))

(event `InputAxis|PowerDownLeft`
  (params (AxisValue :type "Float (single-precision)"))
  (set `self.LeftPower` (`KismetMathLibrary.FClamp` (- (`self.LeftPower`) AxisValue) 1.0 10.0)))

(event `InputAxis|CrosshairY`
  (params (AxisValue :type "Float (single-precision)"))
  (bind (_relativelocation_x _relativelocation_y) (`KismetMathLibrary.BreakVector` (`SceneComponent.RelativeLocation` (`self.Crosshair`))))
  (if (and (<= _relativelocation_y 300.0) (>= _relativelocation_y -300.0) (not (`self.Fired`)))
    (`SceneComponent.K2_SetRelativeLocation` (`self.Crosshair`) (`KismetMathLibrary.MakeVector` _relativelocation_x (`KismetMathLibrary.FClamp` (+ _relativelocation_y AxisValue) -300.0 300.0)) false false)
    (goto _label)))

(event `InputAction|ReloadLeft`
  (params (Key :type "Key Structure"))
  (:`Pressed`
    (if (`self.Jammed`)
      _
      (elif (and (`self.ShootLeft`) (not (`self.Reloaded`)))
        (set `self.Reloaded` true)
        (else
          (set `self.Jammed` true)
          (`KismetSystemLibrary.Delay` 3.0)
          (`self.ChooseBulletSide`)
          (set `self.Jammed` false))))))

(event `InputAction|ReloadRight`
  (params (Key :type "Key Structure"))
  (:`Pressed`
    (if (`self.Jammed`)
      _
      (elif (and (not (`self.ShootLeft`)) (not (`self.Reloaded`)))
        (set `self.Reloaded` true)
        (else
          (set `self.Jammed` true)
          (`KismetSystemLibrary.Delay` 3.0)
          (`self.ChooseBulletSide`)
          (set `self.Jammed` false))))))

(event `InputAction|Shoot`
  (params (Key :type "Key Structure"))
  (bind (_loc _rot) (`self.ShootLocation`))
  (:`Pressed`
    (if (`self.Reloaded`)
      (`|SpawnActorFromClass` "/Game/Blueprints/BPA_Bullet.BPA_Bullet_C" (`KismetMathLibrary.MakeTransform` _loc _rot (0.25 0.25 0.25)) "Undefined" "OverrideRootScale" null self null)
      (set `self.Reloaded` false)
      (set `self.Fired` true)
      (`KismetSystemLibrary.Delay` 1.0)
      (`self.ChooseBulletSide`)
      (set `self.Fired` false))))

(event `self.Box.OnComponentBeginOverlap`
  (params (OverlappedComponent :type "PrimitiveComponent Object Reference") (OtherActor :type "Actor Object Reference") (OtherComp :type "PrimitiveComponent Object Reference") (OtherBodyIndex :type Integer) (bFromSweep :type Boolean) (SweepResult :type "HitResult Structure (by ref)"))
  (`GameplayStatics.PlaySound2D` "/Engine/VREditor/Sounds/UI/Teleport_Committed.Teleport_Committed" 1.0 1.0 0.0 null null)
  (`KismetSystemLibrary.Delay` 0.2)
  (`GameplayStatics.OpenLevel` "MainMenu"))

(event `InputAction|FrontLeftThrust`
  (params (Key :type "Key Structure"))
  (:`Pressed`
    (if (`self.CheckAndUseEnergy` (`self.ThrustCost`))
      (`PrimitiveComponent.AddForceAtLocation` (`self.Ship`) (* (`self.GetActorForwardVector`) 2.5) (`SceneComponent.K2_GetComponentLocation` (`self.FrontLeftThrust`)) "None")
      (`ActorComponent.Activate` (`self.LeftThrustParticleSystem1`) false)))
  (:`Released`
    (`ActorComponent.Deactivate` (`self.LeftThrustParticleSystem1`))))

(event `InputAction|FrontRightThrust`
  (params (Key :type "Key Structure"))
  (:`Pressed`
    (if (`self.CheckAndUseEnergy` (`self.ThrustCost`))
      (`PrimitiveComponent.AddForceAtLocation` (`self.Ship`) (* (`self.GetActorForwardVector`) -2.5) (`SceneComponent.K2_GetComponentLocation` (`self.FrontRightThrust`)) "None")
      (`ActorComponent.Activate` (`self.RightThrustParticleSystem`) false)))
  (:`Released`
    (`ActorComponent.Deactivate` (`self.RightThrustParticleSystem`))))

(fn `AccumulateThrusterEnergy`
  (params (IncrementAmount :type Integer))
  (locals (NewLocalVar_0 :type Integer) (NewLocalVar_1 :type Integer))
  (set `self.TotalEnergy` (+ IncrementAmount (`self.TotalEnergy`)))
  (if (not (`KismetMathLibrary.InRange_IntInt` (`self.TotalEnergy`) 0 (`self.MaxEnergy`)))
    (set `self.TotalEnergy` (`self.MaxEnergy`))))

(fn `CheckAndUseEnergy`
  (params (EnergyAmount :type Integer))
  (returns (CanUseThrust :type Boolean))
  (bind _returnvalue (- (`self.TotalEnergy`) EnergyAmount))
  (bind _returnvalue_2 (>= _returnvalue 0))
  (if _returnvalue_2
    (set `self.TotalEnergy` _returnvalue))
  (return _returnvalue_2))

(fn `ChooseBulletSide`
  (if (== (`KismetMathLibrary.RandomInteger` 2) 1)
    (set `self.ShootLeft` true)
    (else
      (set `self.ShootLeft` false))))

(fn `UserConstructionScript`)