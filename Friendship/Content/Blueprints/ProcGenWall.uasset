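; ProcGenWall is a procedural Blueprint that builds a grid of mesh instances on its Wall component.
; The construction script runs nested loops over NumMeshesX and NumMeshesY, adding one instance per cell, offset by MeshWidth along X and MeshLength along Y.
; All instances sit at zero Z with default rotation and scale.
; The event graph holds only disabled placeholder events, so there is no runtime logic.
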(fn `UserConstructionScript`
  (for _index (range (`self.numMeshesX`))
    (for _index_2 (range (`self.numMeshesY`))
      (`InstancedStaticMeshComponent.AddInstance` (`self.Wall`) (`KismetMathLibrary.MakeTransform` (`KismetMathLibrary.MakeVector` (* _index (`self.meshWidth`)) (* _index_2 (`self.meshLength`))))))))